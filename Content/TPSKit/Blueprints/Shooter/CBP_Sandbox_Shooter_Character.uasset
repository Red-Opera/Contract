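; Shooter character Blueprint that extends a parent sandbox character with weapon firing, aiming and sprint feedback through a WeaponManager component.
; Delayed init caches the player camera manager and gives the weapon manager its camera, while IA_Fire input drives firing.
; Tick relays the current weapon's left-hand IK transform through server-to-client events, blocks firing by gait, syncs aim state and toggles sprint camera shake.
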(event Custom|SprintCam
  (bind _characterinputstate (Variables|Default|GetCharacterInputState))
  ;[0 0.03345 0.15 0.5] Sprint Camera Shake
  (if (Utilities|IsValid (Variables|Default|GetPlayer%20Camera%20Manager))
    (if (Math|Boolean|ANDBoolean (.wantstosprint _characterinputstate) (Utilities|Enum|Equal(Enum) (Variables|Default|GetGait) "NewEnumerator2") (not (.wantstoaim _characterinputstate)))
      (CameraShakes|StartCameraShake (Variables|Default|GetPlayer%20Camera%20Manager) "/Game/TPSKit/CameraShakes/SprintCameraShake1.SprintCameraShake1_C" 0.15 "CameraLocal" "0, 0, 0")
      (else
        (Class|PlayerCameraManager|StopAllInstancesOfCameraShake (Variables|Default|GetPlayer%20Camera%20Manager) "/Game/TPSKit/CameraShakes/SprintCameraShake1.SprintCameraShake1_C" false)))))

(event Custom|ClientHandIK
  (params (currentLeftHandIKTransform :type Transform))
  ;[0.5208 0.16 0 0.5] Left Hand IK
  (Variables|Default|SetcurrentLeftHandIKTransform currentLeftHandIKTransform))

(event Custom|SetCameraManager
  ;[0.15 0.15 0.15 0.5] Set player controller variables
  (if (not (Utilities|IsValid (Variables|Default|GetPlayerControllerRef)))
    (bind _asplayer_controller (Utilities|Casting|CastToPlayerController (Pawn|GetController)))
    (bind _output_get (Variables|Default|SetPlayerControllerRef _asplayer_controller))
    (Variables|Default|SetPlayer%20Camera%20Manager (Variables|/Script/Engine.PlayerController|GetPlayerCameraManager _output_get))))

(event Custom|Init
  (Utilities|FlowControl|Delay 0.2)
  (CallFunction|SetCameraManager)
  (Utilities|FlowControl|Delay 0.5)
  (Variables|/Game/TPSKit/Blueprints/Core/WeaponSystem/Components/WeaponManager.WeaponManager_C|SetcameraActor (Variables|Default|GetWeaponManager) (Variables|Default|GetCamera)))

(event Custom|ServerHandIK
  (params (currentLeftHandIKTransform :type Transform))
  ;[0.5208 0.16 0 0.5] Left Hand IK
  (CallFunction|ClientHandIK currentLeftHandIKTransform))

(event Input|EnhancedActionEvents|EnhancedInputActionIA_Fire
  (params (ActionValue :type Boolean) (ElapsedSeconds :type Float%20%28double-precision%29) (TriggeredSeconds :type Float%20%28double-precision%29) (InputAction :type Input%20Action%20Object%20Reference :default "/Game/TPSKit/Input/IA_Fire.IA_Fire"))
  (:Triggered
    (Default|FireWeapon (Variables|Default|GetWeaponManager) ActionValue))
  (:Canceled
    (Default|FireWeapon (Variables|Default|GetWeaponManager) false :!label _label))
  (:Completed
    (goto _label)))

(event EventBeginPlay
  (|CallParentFunction)
  (CallFunction|Init))

(event Collision|EventActorBeginOverlap
  (params (OtherActor :type Actor%20Object%20Reference)))

(event EventTick
  (params (DeltaSeconds :type Float%20%28single-precision%29))
  (bind _weaponmanager (Variables|Default|GetWeaponManager))
  (|CallParentFunction DeltaSeconds)
  (Utilities|FlowControl|Sequence
    (:then_0
      ;[0.5208 0.16 0 0.5] Left Hand IK
      (if (!= (Variables|/Game/TPSKit/Blueprints/Core/WeaponSystem/Components/WeaponManager.WeaponManager_C|GetCurrentWeaponIndex (Variables|Default|GetWeaponManager)) -1)
        (CallFunction|ServerHandIK (Variables|/Game/TPSKit/Blueprints/Core/WeaponSystem/WeaponData/WeaponData_BP.WeaponData_BP_C|GetLeftHandIK (Utilities|Array|Get(acopy) (Variables|/Game/TPSKit/Blueprints/Core/WeaponSystem/Components/WeaponManager.WeaponManager_C|GetWeaponSlots _weaponmanager) (Variables|/Game/TPSKit/Blueprints/Core/WeaponSystem/Components/WeaponManager.WeaponManager_C|GetCurrentWeaponIndex _weaponmanager))))))
    (:then_1
      ;[0.625 0 0.04496 0.5] Don't allow shooting when sprinting
      (Variables|/Game/TPSKit/Blueprints/Core/WeaponSystem/Components/WeaponManager.WeaponManager_C|SetcanFireWeapon (Variables|Default|GetWeaponManager) (not (Utilities|Enum|Equal(Enum) (Variables|Default|GetGait) "NewEnumerator2"))))
    (:then_2
      ;[0.02624 0.06663 0.08866] Update aiming in weapon manager
      (Variables|/Game/TPSKit/Blueprints/Core/WeaponSystem/Components/WeaponManager.WeaponManager_C|Setaiming (Variables|Default|GetWeaponManager) (.WantsToAim (Utilities|Struct|BreakCharacterInputState (Variables|Default|GetCharacterInputState)))))
    (:then_3
      (CallFunction|SprintCam))))

(fn ConstructionScript
  (|CallParentFunction))
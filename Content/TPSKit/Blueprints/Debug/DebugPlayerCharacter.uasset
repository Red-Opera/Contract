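; Debug component for a player character that shows health, armor and weapon info on screen.
; On BeginPlay it caches the owner's WeaponManager and HealthComponent, then creates a W_PlayerDebugger widget for the owning pawn's PlayerController and adds it to the viewport.
; Every Tick it polls those components and pushes their current state to the widget, without checking that the widget was created.
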(event EventBeginPlay
  (bind _returnvalue (Components|GetOwner))
  (Variables|Default|SetWeaponManager (Actor|GetComponentbyClass _returnvalue "/Game/TPSKit/Blueprints/Core/WeaponSystem/Components/WeaponManager.WeaponManager_C"))
  (Variables|Default|SetHealthComponent (Actor|GetComponentbyClass _returnvalue "/Game/TPSKit/Blueprints/Core/HealthSystem/Components/HealthComponent.HealthComponent_C"))
  (bind _aspawn (Utilities|Casting|CastToPawn (Components|GetOwner)))
  (bind _asplayer_controller (Utilities|Casting|CastToPlayerController (Pawn|GetController _aspawn)))
  (bind _returnvalue_2 (UserInterface|CreateWidget "/Game/TPSKit/Blueprints/Debug/W_PlayerDebugger.W_PlayerDebugger_C" _asplayer_controller))
  (bind _output_get (Variables|Default|SetDebugWidget _returnvalue_2))
  (UserInterface|Viewport|AddtoViewport _output_get 0))

(event EventTick
  (params (DeltaSeconds :type Float%20%28single-precision%29))
  (bind _healthcomponent (Variables|Default|GetHealthComponent))
  (Default|UpdateHealthandArmor (Variables|Default|GetDebugWidget) (Variables|/Game/TPSKit/Blueprints/Core/HealthSystem/Components/HealthComponent.HealthComponent_C|Gethealth _healthcomponent) (Variables|/Game/TPSKit/Blueprints/Core/HealthSystem/Components/HealthComponent.HealthComponent_C|Getarmor _healthcomponent))
  (Default|UpdateWeaponInfo (Variables|Default|GetDebugWidget) (Variables|Default|GetWeaponManager)))